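; Pickup item actor that the player can collect into their inventory with the E key.
; Construction script looks up the Tabla_Items row named after the item enum, merges in the instance quantity and applies the mesh.
; Box overlap toggles input and the nearby flag; E adds the item and destroys the actor only if it is the player's selected item.
; ItemSeleccionado toggles custom depth on the mesh for selection highlighting.
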(event `self.ReceiveBeginPlay`)

(event `self.Box.OnComponentBeginOverlap`
  (params (OverlappedComponent :type "PrimitiveComponent Object Reference") (OtherActor :type "Actor Object Reference") (OtherComp :type "PrimitiveComponent Object Reference") (OtherBodyIndex :type Integer) (bFromSweep :type Boolean) (SweepResult :type "HitResult Structure (by ref)"))
  ;[1 1 1] OVerlap
  (cast `/Game/Jugador/PersonajePrincipal_Fausto/Blueprints/Character/Player_BP` OtherActor)
  (`self.EnableInput` (`GameplayStatics.GetPlayerController` 0))
  (set `self.PersonajeCerca` true))

(event `self.Box.OnComponentEndOverlap`
  (params (OverlappedComponent :type "PrimitiveComponent Object Reference") (OtherActor :type "Actor Object Reference") (OtherComp :type "PrimitiveComponent Object Reference") (OtherBodyIndex :type Integer))
  ;[1 1 1] OVerlap
  (cast `/Game/Jugador/PersonajePrincipal_Fausto/Blueprints/Character/Player_BP` OtherActor)
  (`self.DisableInput` (`GameplayStatics.GetPlayerController` 0))
  (set `self.PersonajeCerca` false))

(event `Key|E`
  (params (Key :type "Key Structure"))
  ;[1 1 1] Coger Item - Llenar diccionario
  (:`Pressed`
    (bind _asplayer_bp (cast `/Game/Jugador/PersonajePrincipal_Fausto/Blueprints/Character/Player_BP` (`GameplayStatics.GetPlayerPawn` 0)))
    (if (== (`/Game/Jugador/PersonajePrincipal_Fausto/Blueprints/Character/Player_BP.ItemSeleccionado` _asplayer_bp) self)
      (`/Game/Jugador/PersonajePrincipal_Fausto/Blueprints/Character/Player_BP.AgregarItem` _asplayer_bp (`self.InformacionCompleta`))
      (`self.K2_DestroyActor`))))

(fn `ItemSeleccionado`
  (params (Selecionado :type Boolean))
  (`PrimitiveComponent.SetRenderCustomDepth` (`self.Modelo`) Selecionado))

(fn `ObtenerInformacionCompleta`
  (params (Informacion :type "/Game/Jugador/Inventario/Estructura_Item Structure"))
  (returns (InformacionCompleta :type "/Game/Jugador/Inventario/Estructura_ItemCompleta Structure"))
  (locals (NewLocalVar_0 :type "/Game/Jugador/Inventario/Estructura_ItemCompleta Structure"))
  ;[1 1 1] vemos si existe el item
  (bind _returnvalue (`|GetDataTableRow` "/Game/Jugador/Inventario/Tabla_Items.Tabla_Items" (`KismetStringLibrary.Conv_StringToName` (`|GetEnumeratorNameAsString` Informacion_Item_2_F9E6201E44E0BBAC2C4AF9B5BCC63433)))
    (:`then`
      ;[1 1 1] actualizo la estructura ..
      (bind _structout (setmembers `/Game/Jugador/Inventario/Estructura_ItemCompleta` :`StructRef` _returnvalue :`Cantidad` Informacion_Cantidad_5_A244BEBC4D70F6892155E59C25E5D7F9))
      (return _structout))))

(fn `UserConstructionScript`
  (bind _informacioncompleta (`self.ObtenerInformacionCompleta` (`self.Informacion`)))
  (bind _output_get (set `self.InformacionCompleta` _informacioncompleta))
  (`StaticMeshComponent.SetStaticMesh` (`self.Modelo`) (`.Malla_30_86A069D74BA230A3D48ED998BC884784` (break `/Game/Jugador/Inventario/Estructura_ItemCompleta` _output_get))))