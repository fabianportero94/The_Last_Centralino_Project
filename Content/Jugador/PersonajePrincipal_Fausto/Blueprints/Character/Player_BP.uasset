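; Player character Blueprint for the main character Fausto, handling look, movement, sprint and weapon toggle input.
; Movement follows control yaw, and look input is scaled down before driving controller pitch and yaw.
; Sprint input sets EstaCorriendo, which a shared function turns into walk or run MaxWalkSpeed; moving backward cancels sprint.
; Pistol and knife inputs only flip independent booleans, and BeginPlay shows the FPS counter.
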(event `InputAction|ConPistola`
  (params (Key :type "Key Structure"))
  ;[1 1 1] Con Arma
  (:`Pressed`
    (set `self.Presionando2` (not (`self.Presionando2`)))))

(event `InputAxis|LookPitch`
  (params (AxisValue :type "Float (single-precision)"))
  ;[1 1 1] Entrada Raton
  (`self.AddControllerPitchInput` (* AxisValue 0.2)))

(event `self.ReceiveBeginPlay`
  (`KismetSystemLibrary.ExecuteConsoleCommand` "Stat FPS" null))

(event `InputAction|Correr`
  (params (Key :type "Key Structure"))
  ;[1 1 1] Correr
  (:`Pressed`
    (set `self.estaCorriendo` true)
    (`self.Actualizacion de velociadad de movimiento` :!label _label))
  (:`Released`
    (set `self.estaCorriendo` false)
    (goto _label)))

(event `InputAction|conCuchillo`
  (params (Key :type "Key Structure"))
  ;[1 1 1] Con Arma
  (:`Pressed`
    (set `self.Presionando1` (not (`self.Presionando1`)))))

(event `InputAxis|LookYaw`
  (params (AxisValue :type "Float (single-precision)"))
  ;[1 1 1] Entrada Raton
  (`self.AddControllerYawInput` (* AxisValue 0.2)))

(event `InputAxis|MoveForward`
  (params (AxisValue :type "Float (single-precision)"))
  ;[1 1 1] Entrada de Movimientos
  (bind _output_get (set `self.Valor_MoveForward` AxisValue))
  (`self.AddMovementInput` (`KismetMathLibrary.GetForwardVector` (`KismetMathLibrary.MakeRotator` 0.0 0.0 (.yaw (`self.GetControlRotation`)))) _output_get)
  ;;[1 1 1] Hacia atras shift se deshabilita
  (if (and (<= _output_get -0.1) (`self.estaCorriendo`))
    (set `self.estaCorriendo` false)
    (`self.Actualizacion de velociadad de movimiento`)))

(event `InputAxis|MoveRight`
  (params (AxisValue :type "Float (single-precision)"))
  ;[1 1 1] Entrada de Movimientos
  (`self.AddMovementInput` (`KismetMathLibrary.GetRightVector` (`KismetMathLibrary.MakeRotator` 0.0 0.0 (.yaw (`self.GetControlRotation`)))) AxisValue))

(fn `Actualizacion de velociadad de movimiento`
  (bind _charactermovement (`self.CharacterMovement`))
  (if (`self.estaCorriendo`)
    (set `CharacterMovementComponent.MaxWalkSpeed` 350.0 _charactermovement)
    (else
      (set `CharacterMovementComponent.MaxWalkSpeed` 170.0 _charactermovement))))

(fn `UserConstructionScript`)