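; Player character with a toggled revolver and knife, flashlight, sprint, aim zoom, distraction whistle and widget HUD.
; The revolver fires camera hitscan traces, while the knife plays montages and traces between sockets during attacks.
; Tick drives aimed body rotation through Player_AnimBP, footsteps, item highlighting and the health bar.
; A map-based inventory adds, uses and drops items; death triggers a random animation, slow motion and camera blend.
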(event `InputAction|Atacar`
  (params (Key :type "Key Structure"))
  (bind _returnvalue (`GameplayStatics.GetPlayerCameraManager` 0))
  (bind _returnvalue_2 (`self.K2_GetActorLocation` _returnvalue))
  ;[1 1 1] Disparos Revolver
  (:`Pressed`
    (if (> (`self.CantidadBalas`) 0)
      (if (and (`self.Presionado2_Revolver`) (`self.Apuntando`))
        (bind _outhit (`KismetSystemLibrary.LineTraceSingle` :`Start` _returnvalue_2 :`End` (+ _returnvalue_2 (* (`self.GetActorForwardVector` _returnvalue) 5000)) :`TraceChannel` "TraceTypeQuery2" :`DrawDebugType` "ForDuration"))
        (set `self.CantidadBalas` (- (`self.CantidadBalas`) 1))
        ;;[1 1 1] Sonido Disparos
        (`GameplayStatics.SpawnSoundAtLocation` "/Game/Sonidos/Personaje_Principal/Ataque/Pistola/Balazopiel.Balazopiel" (`self.K2_GetActorLocation`) (struct) 1.0 1.0 0.0 null null false)
        (`KismetSystemLibrary.PrintString` (`KismetSystemLibrary.GetDisplayName` (`.HitActor` (`GameplayStatics.BreakHitResult` _outhit))))
        (`AISense_Damage.ReportDamageEvent` (`.HitActor` (`GameplayStatics.BreakHitResult` _outhit)) self 1.0 (`.TraceStart` (`GameplayStatics.BreakHitResult` _outhit)) (`.Location` (`GameplayStatics.BreakHitResult` _outhit)))
        (`GameplayStatics.ApplyDamage` (`.HitActor` (`GameplayStatics.BreakHitResult` _outhit)) 50.0 (`self.GetInstigatorController` self) self "/Script/Engine.DamageType")))))

(event `InputAction|ConPistola`
  (params (Key :type "Key Structure"))
  ;[1 1 1] Con Arma
  (:`Pressed`
    (bind _output_get (set `self.Presionado2_Revolver` (not (`self.Presionado2_Revolver`))))
    (if _output_get
      (`self.PlayAnimMontage` "/Game/Jugador/PersonajePrincipal_Fausto/MIxamoLucho/Knife_walking/knife_Unarmed_Equip_Underarm_Montage.knife_Unarmed_Equip_Underarm_Montage")
      (`|ExecutionSequence`
        (:`then_0`
          (`KismetSystemLibrary.Delay` 0.4)
          ;;[1 1 1] Sonido Sacar y guardar pistola
          (`GameplayStatics.SpawnSoundAtLocation` "/Game/Sonidos/Personaje_Principal/Ataque/Pistola/cargar_arma.cargar_arma" (`self.K2_GetActorLocation`) (struct) 1.0 1.0 0.0 null null false))
        (:`then_1`
          ;;[1 1 1] Desenfundar Revolver
          (`KismetSystemLibrary.Delay` 0.4)
          (`self.DesenfundarArma` (`self.Revolver`) (`self.Mesh`) "RightHandSocket_0")
          ;[1 1 1] Cuando un arma se activa el resto se desactiva
          (set `self.Presionado1_Cuchillo` false)
          ;;[1 1 1] Enfundar Cuchillo
          (`SceneComponent.SetVisibility` (`self.Cuchillo`) false false :!label _label)))
      (else
        (`self.PlayAnimMontage` "/Game/Jugador/PersonajePrincipal_Fausto/MIxamoLucho/Knife_walking/knife_standing_disarm_underarm_Montage.knife_standing_disarm_underarm_Montage")
        (`|ExecutionSequence`
          (:`then_0`
            (`KismetSystemLibrary.Delay` 0.4)
            (`GameplayStatics.SpawnSoundAtLocation` "/Game/Sonidos/Personaje_Principal/Ataque/Pistola/GuardarArma.GuardarArma" (`self.K2_GetActorLocation`) (struct) 1.0 1.0 0.0 null null false))
          (:`then_1`
            ;;[1 1 1] Enfundar Revolver
            (`KismetSystemLibrary.Delay` 0.4)
            (`SceneComponent.SetVisibility` (`self.Revolver`) false false :!label _label_2)))))))

(event `InputAction|conCuchillo`
  (params (Key :type "Key Structure"))
  ;[1 1 1] Con Arma
  (:`Pressed`
    (bind _output_get (set `self.Presionado1_Cuchillo` (not (`self.Presionado1_Cuchillo`))))
    (if _output_get
      (`self.PlayAnimMontage` "/Game/Jugador/PersonajePrincipal_Fausto/MIxamoLucho/Knife_walking/knife_Unarmed_Equip_Underarm_Montage.knife_Unarmed_Equip_Underarm_Montage")
      (`|ExecutionSequence`
        (:`then_0`
          (`KismetSystemLibrary.Delay` 0.4)
          ;;[1 1 1] Sonido Sacar y Guardar Cuchillo
          (`GameplayStatics.SpawnSoundAtLocation` "/Game/Sonidos/Personaje_Principal/Ataque/Cuchillo/SacarCuchillo.SacarCuchillo" (`self.K2_GetActorLocation`) (struct) 1.0 1.0 0.0 null null false))
        (:`then_1`
          ;;[1 1 1] Desenfundar Cuchillo
          (`KismetSystemLibrary.Delay` 0.4)
          (`self.DesenfundarArma` (`self.Cuchillo`) (`self.Mesh`) "RightHandSocket")
          ;[1 1 1] Cuando un arma se activa el resto se desactiva
          (set `self.Presionado2_Revolver` false)
          (goto _label_2)))
      (else
        (`self.PlayAnimMontage` "/Game/Jugador/PersonajePrincipal_Fausto/MIxamoLucho/Knife_walking/knife_standing_disarm_underarm_Montage.knife_standing_disarm_underarm_Montage")
        (`|ExecutionSequence`
          (:`then_0`
            (`KismetSystemLibrary.Delay` 0.4)
            (`GameplayStatics.SpawnSoundAtLocation` "/Game/Sonidos/Personaje_Principal/Ataque/Cuchillo/GuardarCuchillo.GuardarCuchillo" (`self.K2_GetActorLocation`) (struct) 1.0 1.0 0.0 null null false))
          (:`then_1`
            ;;[1 1 1] Enfundar Cuchillo
            (`KismetSystemLibrary.Delay` 0.4)
            (goto _label)))))))

(event `Key|Q`
  (params (Key :type "Key Structure"))
  ;[1 1 1] Linterna
  (:`Pressed`
    (bind _output_get (set `self.SW_Linterna` (not (`self.SW_Linterna`))))
    (`SceneComponent.SetVisibility` (`self.Linterna`) _output_get false)))

(event `InputAction|Atacar`
  (params (Key :type "Key Structure"))
  (bind _returnvalue (`AnimInstance.IsAnyMontagePlaying` (`SkeletalMeshComponent.GetAnimInstance` (`self.Mesh`))))
  ;[1 1 1] Atacar
  ;;[1 1 1] Animacion
  (:`Pressed`
    (if (`self.Presionado1_Cuchillo`)
      (if (and (== (`self.Valor_MoveForward`) 0.0) (== (`self.Valor_MoveRight`) 0.0))
        (`|ExecutionSequence`
          (:`then_0`
            (if (`self.Apuntando`)
              (if (not _returnvalue)
                (`|PlayMontage` (`self.Mesh`) "/Game/Jugador/PersonajePrincipal_Fausto/MIxamoLucho/Knife_Atack/Knife_Ataque_Apuntando_Lucho_Montage.Knife_Ataque_Apuntando_Lucho_Montage"
                  (:`then`
                    (`KismetSystemLibrary.RetriggerableDelay` 1.0))))))
          (:`then_1`
            (if (not _returnvalue)
              (`|PlayMontage` (`self.Mesh`) "/Game/Jugador/PersonajePrincipal_Fausto/MIxamoLucho/Knife_Atack/knife_Standing_Melee_Attack_Horizontal_Montage_SlotDefault.knife_Standing_Melee_Attack_Horizontal_Montage_SlotDefault"
                (:`then`
                  (`KismetSystemLibrary.RetriggerableDelay` 0.5)
                  ;;[1 1 1] Sonido Cuchillo
                  (`GameplayStatics.SpawnSoundAtLocation` "/Game/Sonidos/Personaje_Principal/Ataque/Cuchillo/AtaqueZombiet.AtaqueZombiet" (`self.K2_GetActorLocation`) (struct) 1.0 1.0 0.0 null null false))))))
        (elif (not _returnvalue)
          (`|PlayMontage` (`self.Mesh`) "/Game/Jugador/PersonajePrincipal_Fausto/MIxamoLucho/Knife_Atack/knife_Standing_Melee_Attack_Horizontal_MOvimiento_Montage.knife_Standing_Melee_Attack_Horizontal_MOvimiento_Montage"
            (:`then`
              (`KismetSystemLibrary.RetriggerableDelay` 1.0))))))))

(event `self.ReceiveTick`
  (params (DeltaSeconds :type "Float (single-precision)"))
  (bind (_returnvalue_roll _returnvalue_pitch) (`KismetMathLibrary.BreakRotator` (`self.GetControlRotation`)))
  (bind _returnvalue (`self.K2_GetActorLocation`))
  (bind _itemseleccionado (`self.ItemSeleccionado`))
  (bind _camera (`self.Camera`))
  (bind _returnvalue_2 (`SceneComponent.K2_GetComponentLocation` _camera))
  (bind _returnvalue_3 (`SkeletalMeshComponent.GetAnimInstance` (`self.Mesh`)))
  (bind _returnvalue_4 (`PlayerCameraManager.GetCameraLocation` (`GameplayStatics.GetPlayerCameraManager` 0)))
  (bind _returnvalue_5 (`KismetMathLibrary.VSize` (`MovementComponent.Velocity` (`self.CharacterMovement`))))
  ;[1 1 1] EVENT TICK
  (`|ExecutionSequence`
    (:`then_0`
      ;[1 1 1] Linterna
      (`SceneComponent.K2_SetRelativeRotation` (`self.Linterna`) (`KismetMathLibrary.MakeRotator` 0.0 _returnvalue_pitch 90.0) false false))
    (:`then_1`
      ;[1 1 1] Atacar
      ;;[1 1 1] Rastreo Dano Cuchillo
      (if (`self.RealizandoAtaque`)
        (`|ExecutionSequence`
          (:`then_0`
            (`self.RastreoDano` "SocketCuchilloInicio" "SocketCuchilloFinal"))
          (:`then_1`
            (`self.RastreoDano` "SocketCuchilloApuntandoInicio" "SocketCuchilloApuntandoFinal")))))
    (:`then_2`
      ;[1 1 1] Rotacion del cuerpo respecto al mouse, solo cuando apunta con el revolver
      (if (and (or (`self.Presionado1_Cuchillo`) (`self.Presionado2_Revolver`)) (`self.Apuntando`))
        (cast `/Game/Jugador/PersonajePrincipal_Fausto/Blueprints/Character/Player_AnimBP` _returnvalue_3)
        (`self.RotacionCabeza`)
        (else
          (bind _asplayer_anim_bp (cast `/Game/Jugador/PersonajePrincipal_Fausto/Blueprints/Character/Player_AnimBP` _returnvalue_3))
          (set `/Game/Jugador/PersonajePrincipal_Fausto/Blueprints/Character/Player_AnimBP.RotacionCuerpo` (struct) _asplayer_anim_bp))))
    (:`then_3`
      ;[1 1 1] sonido
      (if (not (< _returnvalue_5 30.0))
        (`KismetSystemLibrary.Delay` (`KismetMathLibrary.MapRangeClamped` _returnvalue_5 0.0 360.0 1.0 0.4))
        (if (< _returnvalue_5 30.0)
          _
          (elif (not (`NavMovementComponent.IsFalling` (`self.CharacterMovement`)))
            (bind (_outhits _returnvalue_6) (`KismetSystemLibrary.LineTraceMulti` _returnvalue_4 (- _returnvalue_4 (0.0 0.0 1000.0)) "TraceTypeQuery1"))
            (if _returnvalue_6
              (`GameplayStatics.SpawnSoundAtLocation` "/Game/Sonidos/Personaje_Principal/Pasos/SonidosPasos.SonidosPasos" _returnvalue (struct) 1.0 1.0 0.0 null null)
              (`GameplayStatics.SpawnSoundAtLocation` null _returnvalue (struct) 1.0 1.0 0.0 null null))))))
    (:`then_4`
      ;[1 1 1] Inventario
      (bind (_outhit _returnvalue_7) (`KismetSystemLibrary.LineTraceSingle` _returnvalue_2 (+ _returnvalue_2 (* (`KismetMathLibrary.GetForwardVector` (`SceneComponent.K2_GetComponentRotation` _camera)) 5000.0)) "TraceTypeQuery1"))
      (if _returnvalue_7
        (bind _asitem_bp (cast `/Game/Jugador/Inventario/Item_BP` (`.HitActor` (`GameplayStatics.BreakHitResult` _outhit)))
          (:`then`
            (if (`/Game/Jugador/Inventario/Item_BP.PersonajeCerca` _asitem_bp)
              (if (not (== _asitem_bp (`self.ItemSeleccionado`)))
                (bind _output_get (set `self.ItemSeleccionado` _asitem_bp))
                (`/Game/Jugador/Inventario/Item_BP.ItemSeleccionado` _output_get true))))
          (:`CastFailed`
            (`/Engine/EditorBlueprintResources/StandardMacros.IsValid` _itemseleccionado :!label _label_3
              (:`Is Valid`
                (`/Game/Jugador/Inventario/Item_BP.ItemSeleccionado` _itemseleccionado false)
                (set `self.ItemSeleccionado` null)))))
        (else
          (goto _label_3))))
    (:`then_5`
      ;[1 1 1] WidgetSalud
      (bind _assalud_personaje_wbp (cast `/Game/UI/UI_Blueprints/Salud_Personaje_WBP` (`self.WidgetSalud`)))
      (`ProgressBar.SetPercent` (`/Game/UI/UI_Blueprints/Salud_Personaje_WBP.ProgressBar_35` _assalud_personaje_wbp) (/ (`self.Salud`) 100.0)))))

(event `InputAxis|LookPitch`
  (params (AxisValue :type "Float (single-precision)"))
  ;[1 1 1] Entrada Raton
  (`self.AddControllerPitchInput` (* AxisValue 0.2)))

(event `InputAction|Correr`
  (params (Key :type "Key Structure"))
  ;[1 1 1] Correr
  (:`Pressed`
    (set `self.estaCorriendo` true)
    (`self.Actualizacion de velociadad de movimiento` :!label _label_4))
  (:`Released`
    (set `self.estaCorriendo` false)
    (goto _label_4)))

(event `InputAxis|LookYaw`
  (params (AxisValue :type "Float (single-precision)"))
  ;[1 1 1] Entrada Raton
  (`self.AddControllerYawInput` (* AxisValue 0.2)))

(event `self.ReceiveBeginPlay`
  ;[1 1 1] BeginPlay
  (`KismetSystemLibrary.ExecuteConsoleCommand` "Stat FPS" null)
  (bind _returnvalue (`|CreateWidget` "/Game/UI/UI_Blueprints/Puntero.Puntero_C"))
  (`UserWidget.AddToPlayerScreen` _returnvalue 0)
  (bind _returnvalue_2 (`|CreateWidget` "/Game/UI/UI_Blueprints/WidgetInventario_BP.WidgetInventario_BP_C" (`GameplayStatics.GetPlayerController` 0)))
  (set `self.WidgetInventario` _returnvalue_2)
  (bind _returnvalue_3 (`|CreateWidget` "/Game/UI/UI_Blueprints/Salud_Personaje_WBP.Salud_Personaje_WBP_C"))
  (bind _output_get (set `self.WidgetSalud` _returnvalue_3))
  (`UserWidget.AddToPlayerScreen` _output_get 0)
  (bind _returnvalue_4 (`|CreateWidget` "/Game/UI/UI_Blueprints/WidgetMuniciones.WidgetMuniciones_C"))
  (bind _output_get_2 (set `self.WidgetBalas` _returnvalue_4))
  (`UserWidget.AddToPlayerScreen` _output_get_2 0))

(event `InputAxis|MoveForward`
  (params (AxisValue :type "Float (single-precision)"))
  ;[1 1 1] Entrada de Movimientos
  (bind _output_get (set `self.Valor_MoveForward` AxisValue))
  (`self.AddMovementInput` (`KismetMathLibrary.GetForwardVector` (`KismetMathLibrary.MakeRotator` 0.0 0.0 (.yaw (`self.GetControlRotation`)))) _output_get)
  ;;[1 1 1] Hacia atras shift se deshabilita
  (if (and (<= _output_get -0.1) (`self.estaCorriendo`))
    (set `self.estaCorriendo` false)
    (`self.Actualizacion de velociadad de movimiento`)))

(event `InputAxis|MoveRight`
  (params (AxisValue :type "Float (single-precision)"))
  ;[1 1 1] Entrada de Movimientos
  (bind _output_get (set `self.Valor_MoveRight` AxisValue))
  (`self.AddMovementInput` (`KismetMathLibrary.GetRightVector` (`KismetMathLibrary.MakeRotator` 0.0 0.0 (.yaw (`self.GetControlRotation`)))) _output_get))

(event `Key|CapsLock`
  (params (Key :type "Key Structure"))
  ;[1 1 1] Inventario
  ;;[1 1 1] Abrir widget inventario
  (:`Pressed`
    (`self.MostrarInventario` true)))

(event `self.ReceiveAnyDamage`
  (params (Damage :type "Float (single-precision)") (DamageType :type "DamageType Object Reference") (InstigatedBy :type "Controller Object Reference") (DamageCauser :type "Actor Object Reference"))
  ;[1 1 1] Dano
  (`self.Muerte`)
  (set `self.Salud` (`KismetMathLibrary.FClamp` (- (`self.Salud`) Damage) 0.0 100.0)))

(event `InputAction|Apuntar`
  (params (Key :type "Key Structure"))
  (bind _returnvalue (`GameplayStatics.GetPlayerCameraManager` 0))
  (bind _returnvalue_2 (`GameplayStatics.GetPlayerCameraManager` 0))
  ;[1 1 1] Apuntar
  (:`Pressed`
    (set `self.Apuntando` true)
    ;;[1 1 1] Se limita la rotacion cuando esta con un arma
    (set `PlayerCameraManager.ViewPitchMax` 25.0 _returnvalue)
    (set `PlayerCameraManager.ViewPitchMin` -50.0 _returnvalue)
    (if (or (`self.Presionado1_Cuchillo`) (`self.Presionado2_Revolver`))
      (bind (_direction _set_field_of_view) (`Timeline|Apuntar_Timeline` :!label _label_5)
        (:`Update`
          (`CameraComponent.SetFieldOfView` (`self.Camera`) _set_field_of_view)))))
  (:`Released`
    (set `self.Apuntando` false)
    (set `PlayerCameraManager.ViewPitchMax` 90.0 _returnvalue_2)
    (set `PlayerCameraManager.ViewPitchMin` -90.0 _returnvalue_2)
    (goto _label_5 :!via `Reverse`)))

(event `Muerte`
  ;[1 1 1] Dano
  (if (== (`self.Salud`) 0.0)
    (`SkeletalMeshComponent.PlayAnimation` (`self.Mesh`) (select `int` (`KismetMathLibrary.RandomIntegerInRange` 0 3) :`0` "/Game/Jugador/PersonajePrincipal_Fausto/MIxamoLucho/Muerte/Flying_Back_Death_Montage.Flying_Back_Death_Montage" :`1` "/Game/Jugador/PersonajePrincipal_Fausto/MIxamoLucho/Muerte/Dying__1_.Dying__1_" :`2` "/Game/Jugador/PersonajePrincipal_Fausto/MIxamoLucho/Muerte/Standing_React_Death_Backward__1___1_.Standing_React_Death_Backward__1___1_" :`3` "/Game/Jugador/PersonajePrincipal_Fausto/MIxamoLucho/Muerte/Standing_Death_Forward_01__2_.Standing_Death_Forward_01__2_" :!type "AnimationAsset Object Reference") false)
    (`self.SetActorTickEnabled` false)
    (`self.Camara de Muerte`)
    (`GameplayStatics.SetGlobalTimeDilation` 0.5)))

(event `self.Box.OnComponentBeginOverlap`
  (params (OverlappedComponent :type "PrimitiveComponent Object Reference") (OtherActor :type "Actor Object Reference") (OtherComp :type "PrimitiveComponent Object Reference") (OtherBodyIndex :type Integer) (bFromSweep :type Boolean) (SweepResult :type "HitResult Structure (by ref)"))
  ;[1 1 1] No sirve pero esta porsiaca - Fausto
  (bind _aszombie_pawn_bp (cast `/Game/Enemigos/Enemigo_Blueprints/Zombie_Pawn_BP` OtherActor))
  (set `self.Acuchillado` true))

(event `InputAction|Distraer`
  (params (Key :type "Key Structure"))
  (bind _returnvalue (`self.K2_GetActorLocation`))
  (:`Pressed`
    (`GameplayStatics.PlaySoundAtLocation` "/Game/Sonidos/silbido_distract.silbido_distract" _returnvalue (struct) 1.0 1.0 0.0 null null null)
    (`AISense_Hearing.ReportNoiseEvent` _returnvalue 1.0 self 0.0 "Noise")))

(event `self.Box.OnComponentEndOverlap`
  (params (OverlappedComponent :type "PrimitiveComponent Object Reference") (OtherActor :type "Actor Object Reference") (OtherComp :type "PrimitiveComponent Object Reference") (OtherBodyIndex :type Integer))
  ;[1 1 1] No sirve pero esta porsiaca - Fausto
  (cast `/Game/Enemigos/Enemigo_Blueprints/Zombie_Pawn_BP` OtherActor)
  (set `self.Acuchillado` false))

(fn `Actualizacion de velociadad de movimiento`
  (bind _charactermovement (`self.CharacterMovement`))
  (if (`self.estaCorriendo`)
    (set `CharacterMovementComponent.MaxWalkSpeed` 350.0 _charactermovement)
    (else
      (set `CharacterMovementComponent.MaxWalkSpeed` 170.0 _charactermovement))))

(fn `AgregarItem`
  (params (Item :type "/Game/Jugador/Inventario/Estructura_ItemCompleta Structure"))
  (bind (_value _returnvalue) (`BlueprintMapLibrary.Map_Find` (`self.Inventario`) Item_ClaveItem_32_0F205E5243C67CEF4FE9C4B78A682B16))
  (if _returnvalue
    (bind _structout (setmembers `/Game/Jugador/Inventario/Estructura_ItemCompleta` :`StructRef` _value :`Cantidad` (+ (`.Cantidad_7_D3FC781F4A30B5DFC0B2A4825EB2CB01` (break `/Game/Jugador/Inventario/Estructura_ItemCompleta` _value)) Item_Cantidad_7_D3FC781F4A30B5DFC0B2A4825EB2CB01)))
    (`BlueprintMapLibrary.Map_Add` (`self.Inventario`) Item_ClaveItem_32_0F205E5243C67CEF4FE9C4B78A682B16 _structout)
    (else
      (`BlueprintMapLibrary.Map_Add` (`self.Inventario`) Item_ClaveItem_32_0F205E5243C67CEF4FE9C4B78A682B16 (`local.Item`)))))

(fn `Camara de Muerte`
  (`PlayerController.SetViewTargetWithBlend` (`GameplayStatics.GetPlayerController` 0) (`ChildActorComponent.ChildActor` (`self.CamaraMuerte_ChildActor`)) 5.0 "VTBlend_Cubic" 0.0 true)
  (set `self.bUseControllerRotationYaw` false))

(fn `DesenfundarArma`
  (params (Target :type "StaticMeshComponent Object Reference") (MeshParent :type "SkeletalMeshComponent Object Reference") (NewParam :type Name))
  (`SceneComponent.SetVisibility` Target true false)
  (`SceneComponent.K2_AttachToComponent` Target MeshParent NewParam "SnapToTarget" "SnapToTarget" "SnapToTarget" true))

(fn `MostrarInventario`
  (params (Mostrar :type Boolean))
  (bind _returnvalue (`GameplayStatics.GetPlayerController` 0))
  (bind _widgetinventario (`self.WidgetInventario`))
  (if Mostrar
    (`UserWidget.AddToViewport` _widgetinventario 0)
    (`/Game/UI/UI_Blueprints/WidgetInventario_BP.ConfiguraraInventario` _widgetinventario (`self.Inventario`))
    (set `PlayerController.bShowMouseCursor` true _returnvalue)
    (`WidgetBlueprintLibrary.SetInputMode_UIOnlyEx` _returnvalue _widgetinventario)
    (else
      (`Widget.RemoveFromParent` _widgetinventario)
      (set `PlayerController.bShowMouseCursor` false _returnvalue)
      (`WidgetBlueprintLibrary.SetInputMode_GameOnly` _returnvalue))))

(fn `RastreoDano`
  (params (Nombre_Socket_Inicial :type Name) (Nombre_Socket_Final :type Name))
  (bind _mesh (`self.Mesh`))
  (if (not (`self.ProduciendoDanoCuchillazo`))
    (bind _outhit (`KismetSystemLibrary.LineTraceSingle` :`Start` (`SceneComponent.GetSocketLocation` _mesh Nombre_Socket_Inicial) :`End` (`SceneComponent.GetSocketLocation` _mesh Nombre_Socket_Final) :`TraceChannel` "TraceTypeQuery2" :`DrawDebugType` "ForDuration" :`TraceColor` (struct :`R` 1.0 :`B` 0.760851 :`A` 1.0)))
    (`KismetSystemLibrary.PrintString` (`KismetSystemLibrary.GetDisplayName` (`.HitActor` (`GameplayStatics.BreakHitResult` _outhit))))
    (`AISense_Damage.ReportDamageEvent` (`.HitActor` (`GameplayStatics.BreakHitResult` _outhit)) self 1.0 (`.TraceStart` (`GameplayStatics.BreakHitResult` _outhit)) (`.Location` (`GameplayStatics.BreakHitResult` _outhit)))
    (`GameplayStatics.ApplyDamage` null 75.0 (`self.GetInstigatorController`) self "/Script/Engine.DamageType")))

(fn `RotacionCabeza`
  (bind (_returnvalue_roll _returnvalue_pitch _returnvalue_yaw) (`KismetMathLibrary.BreakRotator` (`self.GetControlRotation`)))
  (bind (_returnvalue_roll_2 _returnvalue_pitch_2 _returnvalue_yaw_2) (`KismetMathLibrary.BreakRotator` (`self.K2_GetActorRotation`)))
  (bind (_returnvalue_roll_3 _returnvalue_pitch_3 _returnvalue_yaw_3) (`KismetMathLibrary.BreakRotator` (`self.K2_GetActorRotation`)))
  (bind _returnvalue (`KismetMathLibrary.ClampAngle` (- _returnvalue_yaw _returnvalue_yaw_3) -179.899994 -180.0))
  (bind _asplayer_anim_bp (cast `/Game/Jugador/PersonajePrincipal_Fausto/Blueprints/Character/Player_AnimBP` (`SkeletalMeshComponent.GetAnimInstance` (`self.Mesh`))))
  (set `/Game/Jugador/PersonajePrincipal_Fausto/Blueprints/Character/Player_AnimBP.RotacionCuerpo` (`KismetMathLibrary.MakeRotator` (- 0.0 _returnvalue_pitch) 0.0 _returnvalue) _asplayer_anim_bp)
  (if (> _returnvalue 90.0)
    (set `self.RotacionMaxima` 90.0)
    (set `self.RotacionCabezaActor` (+ _returnvalue_yaw_2 (`self.RotacionMaxima`)) :!label _label)
    (elif (< _returnvalue -90.0)
      (set `self.RotacionMaxima` -90.0)
      (goto _label)
      (else
        _)))
  (`self.K2_SetActorRotation` (`KismetMathLibrary.RInterpTo` (`self.K2_GetActorRotation`) (`KismetMathLibrary.MakeRotator` 0.0 0.0 (`self.RotacionCabezaActor`)) (`GameplayStatics.GetWorldDeltaSeconds`) 2.0)))

(fn `SoltarItem`
  (params (Item :type "/Game/Jugador/Inventario/Items Enum" :default "NewEnumerator0"))
  (bind (_returnvalue_x _returnvalue_y) (`KismetMathLibrary.BreakVector` (* (`KismetMathLibrary.RandomUnitVector`) 100.0)))
  (bind _value (`BlueprintMapLibrary.Map_Find` (`self.Inventario`) Item))
  (`|SpawnActorFromClass` "/Game/Jugador/Inventario/Item_BP.Item_BP_C" (`KismetMathLibrary.MakeTransform` (+ (`KismetMathLibrary.MakeVector` _returnvalue_x _returnvalue_y -87.0) (`self.K2_GetActorLocation`))) "Undefined" "OverrideRootScale" null (make `/Game/Jugador/Inventario/Estructura_Item` (break `/Game/Jugador/Inventario/Estructura_ItemCompleta` _value) (`.Cantidad_7_D3FC781F4A30B5DFC0B2A4825EB2CB01` (break `/Game/Jugador/Inventario/Estructura_ItemCompleta` _value))) null)
  (`BlueprintMapLibrary.Map_Remove` (`self.Inventario`) (`local.Item`)))

(fn `UsarItem`
  (params (Item :type "/Game/Jugador/Inventario/Items Enum" :default "NewEnumerator0"))
  (bind (_value _returnvalue) (`BlueprintMapLibrary.Map_Find` (`self.Inventario`) Item))
  (bind (_claveitem _nombre _descripcion _cantidad _imagen _renglon _columna _posicionado _valor) (break `/Game/Jugador/Inventario/Estructura_ItemCompleta` _value))
  (bind _returnvalue_2 (- _cantidad 1.0))
  (if _returnvalue
    (set `self.ValorTemporal` _valor)
    (bind _structout (setmembers `/Game/Jugador/Inventario/Estructura_ItemCompleta` :`StructRef` _value :`Cantidad` _returnvalue_2))
    (if (<= _returnvalue_2 0.0)
      (`BlueprintMapLibrary.Map_Remove` (`self.Inventario`) (`local.Item`))
      (else
        (`BlueprintMapLibrary.Map_Add` (`self.Inventario`) (`local.Item`) _structout)))
    ;[1 1 1] Usar el Item
    (switch `/Game/Jugador/Inventario/Items` (`local.Item`)
      (:`NewEnumerator0`
        (if (<= (`self.CantidadBalas`) 5)
          (set `self.CantidadBalas` (`KismetMathLibrary.Clamp` (+ (`self.CantidadBalas`) (`KismetMathLibrary.FTrunc` (`self.ValorTemporal`))) 0 5))))
      (:`NewEnumerator1`
        (set `self.Salud` (`KismetMathLibrary.FClamp` (+ (`self.Salud`) (`self.ValorTemporal`)) 0.0 100.0)))
      (:`NewEnumerator2`
        (set `self.AbrirPuerta` true))
      (:`NewEnumerator3`
        (`KismetSystemLibrary.PrintString` "Hello")))))

(fn `UserConstructionScript`)