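; Pawn Blueprint for Mufi, an enemy that sets its speed on BeginPlay and performs hand-based melee attacks through inherited functions.
; AtacarMufi checks six attack flags on Mufi_Anim_BP in priority order, covering left, right, two-handed and three combo moves.
; The first active flag selects the hand bone pair and radius passed to Ataque, then is cleared.
; ObtenerPuntos is an empty stub.
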(event `self.ReceiveBeginPlay`
  (`self.Actualizar_Velocidad` 200.0))

(event `self.ReceiveTick`
  (params (DeltaSeconds :type "Float (single-precision)"))
  (`parent.ReceiveTick` DeltaSeconds))

(event `AtacarMufi`
  (bind _mufi_animinstance (`self.Mufi_AnimInstance`))
  (bind _asmufi_anim_bp (cast `/Game/Enemigos/Profes/Mufi/Mufi_Blueprints/Maniquin_Mifu/Mufi_Anim_BP` (`SkeletalMeshComponent.GetAnimInstance` (`self.Mesh`))))
  (bind _output_get (set `self.Mufi_AnimInstance` _asmufi_anim_bp))
  (if (`/Game/Enemigos/Profes/Mufi/Mufi_Blueprints/Maniquin_Mifu/Mufi_Anim_BP.M_AtaqueManoIz` _output_get)
    (set `self.SwitchAtacheMufi` 0)
    (switch `int` (`self.SwitchAtacheMufi`) :!label _label
      (:`0`
        (`self.Ataque` "LeftHandMiddle1" "LeftHandMiddle4" 20.0)
        (set `/Game/Enemigos/Profes/Mufi/Mufi_Blueprints/Maniquin_Mifu/Mufi_Anim_BP.M_AtaqueManoIz` false _mufi_animinstance))
      (:`1`
        (`self.Ataque` "RightHandMiddle1" "RightHandMiddle4" 20.0)
        (set `/Game/Enemigos/Profes/Mufi/Mufi_Blueprints/Maniquin_Mifu/Mufi_Anim_BP.M_AtaqueManoDe` false _mufi_animinstance))
      (:`2`
        (`self.Ataque` "RightHand" "LeftHand" 20.0)
        (set `/Game/Enemigos/Profes/Mufi/Mufi_Blueprints/Maniquin_Mifu/Mufi_Anim_BP.M_Ataque2Manos` false _mufi_animinstance))
      (:`3`
        (`self.Ataque` "RightHandMiddle1" "RightHandMiddle4" 20.0)
        (set `/Game/Enemigos/Profes/Mufi/Mufi_Blueprints/Maniquin_Mifu/Mufi_Anim_BP.M_Combo1` false _mufi_animinstance))
      (:`4`
        (`self.Ataque` "LeftHandMiddle1" "LeftHandMiddle4" 20.0)
        (set `/Game/Enemigos/Profes/Mufi/Mufi_Blueprints/Maniquin_Mifu/Mufi_Anim_BP.M_Combo2` false _mufi_animinstance))
      (:`5`
        (`self.Ataque` "RightHand" "LeftHand" 20.0)
        (set `/Game/Enemigos/Profes/Mufi/Mufi_Blueprints/Maniquin_Mifu/Mufi_Anim_BP.M_Combo3` false _mufi_animinstance)))
    (elif (`/Game/Enemigos/Profes/Mufi/Mufi_Blueprints/Maniquin_Mifu/Mufi_Anim_BP.M_AtaqueManoDe` _output_get)
      (set `self.SwitchAtacheMufi` 1)
      (goto _label)
      (elif (`/Game/Enemigos/Profes/Mufi/Mufi_Blueprints/Maniquin_Mifu/Mufi_Anim_BP.M_Ataque2Manos` _output_get)
        (set `self.SwitchAtacheMufi` 2)
        (goto _label)
        (elif (`/Game/Enemigos/Profes/Mufi/Mufi_Blueprints/Maniquin_Mifu/Mufi_Anim_BP.M_Combo1` _output_get)
          (set `self.SwitchAtacheMufi` 3)
          (goto _label)
          (elif (`/Game/Enemigos/Profes/Mufi/Mufi_Blueprints/Maniquin_Mifu/Mufi_Anim_BP.M_Combo2` _output_get)
            (set `self.SwitchAtacheMufi` 4)
            (goto _label)
            (elif (`/Game/Enemigos/Profes/Mufi/Mufi_Blueprints/Maniquin_Mifu/Mufi_Anim_BP.M_Combo3` _output_get)
              (set `self.SwitchAtacheMufi` 5)
              (goto _label))))))))

(fn `ObtenerPuntos`
  (returns (TargetPoints :type "Array of TargetPoint Object Reference"))
  (return))

(fn `UserConstructionScript`
  (`parent.UserConstructionScript`))