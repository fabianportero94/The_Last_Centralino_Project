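; AI controller for a patrolling NPC, apparently a zombie, that runs NPC_BT and feeds its blackboard.
; On possess it seeds patrol settings from the pawn's PatrolPath.
; Perception stimuli are handled by array index: the first sets CanSeePlayer, while successful second and third ones trigger investigation at the stimulus location, with zombie sounds.
; Muerte stops the behavior tree, sight, hearing and damage senses, and tick on death.
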(event `self.ReceiveBeginPlay`)

(event `self.ReceivePossess`
  (params (PossessedPawn :type "Pawn Object Reference"))
  (bind _returnvalue (`AIBlueprintHelperLibrary.GetBlackboard` null))
  (`self.RunBehaviorTree` "/Game/Enemigos/AI_Blueprints/NPC/NPC_BT.NPC_BT")
  (bind _asnpc_character_bp (cast `/Game/Enemigos/AI_Blueprints/NPC/NPC_BP/NPC_Character_BP` (`self.K2_GetPawn`)))
  (bind _output_get (set `self.MyPawn` _asnpc_character_bp))
  (`BlackboardComponent.SetValueAsBool` _returnvalue "Path_Looping" (`/Game/Enemigos/AI_Blueprints/NPC/Patrol_Path_BP.Is_Looping` (`/Game/Enemigos/AI_Blueprints/NPC/NPC_BP/NPC_Character_BP.PatrolPath` _output_get)))
  (`BlackboardComponent.SetValueAsInt` _returnvalue "Direction" 1)
  (`BlackboardComponent.SetValueAsFloat` _returnvalue "WaitTime" (`/Game/Enemigos/AI_Blueprints/NPC/Patrol_Path_BP.Wait_Time` (`/Game/Enemigos/AI_Blueprints/NPC/NPC_BP/NPC_Character_BP.PatrolPath` (`self.MyPawn`)))))

(event `self.AIPerception.OnPerceptionUpdated`
  (params (UpdatedActors :type "Array of Actor Object Reference (by ref)"))
  (for _array_element UpdatedActors
    (bind _info (`AIPerceptionComponent.GetActorsPerception` (`self.AIPerception`) _array_element))
    (`self.SentidosCompletos` (`.LastSensedStimuli` (break `ActorPerceptionBlueprintInfo` _info)))))

(event `Muerte`
  (bind _aiperception (`self.AIPerception`))
  (`BrainComponent.StopLogic` (`self.BrainComponent`) "Dead")
  (`AIPerceptionComponent.SetSenseEnabled` _aiperception "/Script/AIModule.AISense_Sight" false)
  (`AIPerceptionComponent.SetSenseEnabled` _aiperception "/Script/AIModule.AISense_Hearing" false)
  (`AIPerceptionComponent.SetSenseEnabled` _aiperception "/Script/AIModule.AISense_Damage" false)
  (`self.SetActorTickEnabled` false))

(event `self.AIPerception.OnTargetPerceptionUpdated`
  (params (Actor :type "Actor Object Reference") (Stimulus :type "AIStimulus Structure")))

(fn `SentidosCompletos`
  (params (Array :type "Array of AIStimulus Structure"))
  (locals (LocalSense :type "AIStimulus Structure"))
  (bind _returnvalue (`AIBlueprintHelperLibrary.GetBlackboard` null))
  (bind (_localsense_age _localsense_expirationage _localsense_strength _localsense_stimuluslocation _localsense_receiverlocation _localsense_tag _localsense_bsuccessfullysensed) (break `AIStimulus` (`local.LocalSense`)))
  (bind (_localsense_age_2 _localsense_expirationage_2 _localsense_strength_2 _localsense_stimuluslocation_2 _localsense_receiverlocation_2 _localsense_tag_2 _localsense_bsuccessfullysensed_2) (break `AIStimulus` (`local.LocalSense`)))
  (for (_array_element _array_index) Array
    (set `local.LocalSense` _array_element)
    (switch `int` _array_index
      (:`0`
        (`BlackboardComponent.SetValueAsBool` (`AIBlueprintHelperLibrary.GetBlackboard` null) "CanSeePlayer" _localsense_bsuccessfullysensed_2)
        (`GameplayStatics.PlaySoundAtLocation` "/Game/Sonidos/Zombies/SonidoZombie.SonidoZombie" _localsense_receiverlocation_2 (struct) 1.0 1.0 0.0 null null null))
      (:`1`
        (if _localsense_bsuccessfullysensed_2
          (`GameplayStatics.PlaySoundAtLocation` "/Game/Sonidos/Zombies/SonidoZombie.SonidoZombie" _localsense_receiverlocation_2 (struct) 1.0 1.0 0.0 null null null)
          (`BlackboardComponent.SetValueAsBool` _returnvalue "IsInvestigating" _localsense_bsuccessfullysensed :!label _label)
          (`BlackboardComponent.SetValueAsVector` _returnvalue "TargetLocation" _localsense_stimuluslocation)))
      (:`2`
        (if _localsense_bsuccessfullysensed_2
          (`GameplayStatics.PlaySoundAtLocation` "/Game/Sonidos/Zombies/SonidoZombie.SonidoZombie" _localsense_receiverlocation_2 (struct) 1.0 1.0 0.0 null null null)
          (goto _label))))))

(fn `UserConstructionScript`)