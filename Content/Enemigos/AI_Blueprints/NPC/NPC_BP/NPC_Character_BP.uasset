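; Zombie NPC character that melee-attacks the player, takes damage and dies.
; MeleeAttack plays a random arm montage, while NPC_AtaqueIA reads AnimBP flags to sphere-trace between that limb's sockets and damage Player_BP.
; Tick smoothly turns it toward the player when FacePlayer is set.
; AnyDamage plays hit reactions or, at half of the 100 health cap, stops the AI, plays a death montage, ragdolls and destroys the actor.
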(event `/Game/Enemigos/AI_Blueprints/NPC/NPC_BP/Combat_Interface.MeleeAttack`
  ;[1 1 1] ATAQUE
  (set `self.AtaqueIndex` (`KismetMathLibrary.RandomIntegerInRange` 0 2))
  (`|PlayMontage` (`self.Mesh`) (select `int` (`self.AtaqueIndex`) :`0` "/Game/Enemigos/AI_Blueprints/NPC/NPC_BP/Animaciones/Combate/Montage/NPC_Left_Arm_Attack_Montage.NPC_Left_Arm_Attack_Montage" :`1` "/Game/Enemigos/AI_Blueprints/NPC/NPC_BP/Animaciones/Combate/Montage/NPC_Right_Arm_Attack_Montage.NPC_Right_Arm_Attack_Montage" :`2` "/Game/Enemigos/AI_Blueprints/NPC/NPC_BP/Animaciones/Combate/Montage/NPC_Two_Hands_Attack_M_Montage.NPC_Two_Hands_Attack_M_Montage" :`3` "/Game/Enemigos/AI_Blueprints/NPC/NPC_BP/Animaciones/Combate/Montage/NPC_Patada_Montage.NPC_Patada_Montage" :!type "AnimMontage Object Reference")))

(event `NPC_AtaqueIA`
  (bind _animinstance (`self.AnimInstance`))
  ;[1 1 1] ATAQUE
  (bind _aszombie_npc_anim_bp (cast `/Game/Enemigos/AI_Blueprints/NPC/NPC_BP/Zombie_NPC_AnimBP` (`SkeletalMeshComponent.GetAnimInstance` (`self.Mesh`))))
  (bind _output_get (set `self.AnimInstance` _aszombie_npc_anim_bp))
  (if (`/Game/Enemigos/AI_Blueprints/NPC/NPC_BP/Zombie_NPC_AnimBP.NPC_AtaqueManoIz` _output_get)
    (set `self.SwitchAtaque` 0)
    (switch `int` (`self.SwitchAtaque`) :!label _label
      (:`0`
        (`self.Ataque` "mixamorig_LeftHandMiddle1" "mixamorig_LeftHandMiddle4" 20.0)
        (set `/Game/Enemigos/AI_Blueprints/NPC/NPC_BP/Zombie_NPC_AnimBP.NPC_AtaqueManoIz` false _animinstance))
      (:`1`
        (`self.Ataque` "mixamorig_RightHandMiddle1" "mixamorig_RightHandMiddle4" 20.0)
        (set `/Game/Enemigos/AI_Blueprints/NPC/NPC_BP/Zombie_NPC_AnimBP.NPC_AtaqueManoDe` false _animinstance))
      (:`2`
        (`self.Ataque` "middle_end_left" "middle_end_right" 15.0)
        (set `/Game/Enemigos/AI_Blueprints/NPC/NPC_BP/Zombie_NPC_AnimBP.NPC_Ataque2Manos` false _animinstance))
      (:`3`
        (`self.Ataque` "mixamorig_RightToeBase" "mixamorig_RightToe_End" 15.0)
        (set `/Game/Enemigos/AI_Blueprints/NPC/NPC_BP/Zombie_NPC_AnimBP.NPC_Patada` false _animinstance)))
    (elif (`/Game/Enemigos/AI_Blueprints/NPC/NPC_BP/Zombie_NPC_AnimBP.NPC_AtaqueManoDe` _output_get)
      (set `self.SwitchAtaque` 1)
      (goto _label)
      (elif (`/Game/Enemigos/AI_Blueprints/NPC/NPC_BP/Zombie_NPC_AnimBP.NPC_Ataque2Manos` _output_get)
        (set `self.SwitchAtaque` 2)
        (goto _label)
        (elif (`/Game/Enemigos/AI_Blueprints/NPC/NPC_BP/Zombie_NPC_AnimBP.NPC_Patada` _output_get)
          (set `self.SwitchAtaque` 3)
          (goto _label))))))

(event `Rotacion`
  (params (Delta :type "Float (double-precision)"))
  ;[1 1 1] Interpolacion de Rotación hacia el Player
  (set `self.Delta` Delta)
  (if (`self.FacePlayer`)
    (`self.K2_SetActorRotation` self (`KismetMathLibrary.RInterpTo` (`self.K2_GetActorRotation` self) (`KismetMathLibrary.FindLookAtRotation` (`self.K2_GetActorLocation` self) (`self.K2_GetActorLocation` (`GameplayStatics.GetPlayerCharacter` 0))) (`self.Delta`) 20.0) false)))

(event `self.ReceiveTick`
  (params (DeltaSeconds :type "Float (single-precision)"))
  ;[1 1 1] Interpolacion de Rotación hacia el Player
  (`self.Rotacion` DeltaSeconds))

(event `self.ReceiveBeginPlay`
  ;[1 1 1] Spawn porsiacaso (No sirve)
)

(event `SpawnZombies`
  (bind _nzombies (`self.nZombies`))
  (bind _scale (`self.Scale`))
  ;[1 1 1] Spawn porsiacaso (No sirve)
  (if (> _nzombies 0)
    (for _ (range (+ _nzombies 1))
      (set `self.Scale` (`KismetMathLibrary.RandomFloatInRange` 0.8 1.2))
      (bind _returnvalue (`|SpawnActorFromClass` "/Game/Enemigos/AI_Blueprints/NPC/NPC_BP/NPC_Generico_BP_Child.NPC_Generico_BP_Child_C" (`KismetMathLibrary.MakeTransform` (`NavigationSystemV1.K2_GetRandomLocationInNavigableRadius` (`self.K2_GetActorLocation`) 500.0 null null) (struct) (`KismetMathLibrary.MakeVector` _scale _scale _scale)) "AdjustIfPossibleButAlwaysSpawn" "OverrideRootScale" null (`self.PatrolPath`) true null))
      (`/Engine/EditorBlueprintResources/StandardMacros.IsValid` _returnvalue
        (:`Is Valid`
          (`KismetArrayLibrary.Array_AddUnique` (`self.Seguidores`))
          (set `/Game/Enemigos/AI_Blueprints/NPC/NPC_BP/NPC_Generico_BP_Child.Master` self _returnvalue))))))

(event `self.ReceiveAnyDamage`
  (params (Damage :type "Float (single-precision)") (DamageType :type "DamageType Object Reference") (InstigatedBy :type "Controller Object Reference") (DamageCauser :type "Actor Object Reference"))
  (bind _returnvalue (`self.GetController`))
  ;[1 1 1] Muerte y Dano
  (bind _output_get (set `self.SaludEnemigo` (`KismetMathLibrary.FClamp` (- (`self.SaludEnemigo`) Damage) 0.0 100.0)))
  (if (<= _output_get 50.0)
    (`|ExecutionSequence`
      (:`then_0`
        (bind _asnpc_ai_controller_bp (cast `/Game/Enemigos/AI_Blueprints/NPC/NPC_AI_Controller_BP` _returnvalue))
        (`/Game/Enemigos/AI_Blueprints/NPC/NPC_AI_Controller_BP.Muerte` _asnpc_ai_controller_bp)
        (`Controller.UnPossess` _returnvalue)
        (`Controller.UnPossess` _asnpc_ai_controller_bp))
      (:`then_1`
        (`|PlayMontage` (`self.Mesh`) (select `int` (`KismetMathLibrary.RandomIntegerInRange` 0 2) :`0` "/Game/Enemigos/AI_Blueprints/NPC/NPC_BP/Animaciones/Combate/Muerte/NPC_Muerte_Atras_Montage.NPC_Muerte_Atras_Montage" :`1` "/Game/Enemigos/AI_Blueprints/NPC/NPC_BP/Animaciones/Combate/Muerte/NPC_Muerte_Delante2_Montage.NPC_Muerte_Delante2_Montage" :`2` "/Game/Enemigos/AI_Blueprints/NPC/NPC_BP/Animaciones/Combate/Muerte/NPC_Muerte_Delante_Montage.NPC_Muerte_Delante_Montage" :!type "AnimMontage Object Reference")
          (:`then`
            (`KismetSystemLibrary.Delay` 2.0)
            (`PrimitiveComponent.SetSimulatePhysics` (`self.Mesh`) true)
            (`KismetSystemLibrary.Delay` 10.0)
            (`self.K2_DestroyActor`)))))
    (else
      (`|PlayMontage` (`self.Mesh`) (select `int` (`KismetMathLibrary.RandomIntegerInRange` 0 3) :`0` "/Game/Enemigos/AI_Blueprints/NPC/NPC_BP/Animaciones/Combate/Montage/NPC_Reaction_hit2_Montage.NPC_Reaction_hit2_Montage" :`1` "/Game/Enemigos/AI_Blueprints/NPC/NPC_BP/Animaciones/Combate/Montage/NPC_Reaction_Hit_Montage.NPC_Reaction_Hit_Montage" :`2` "/Game/Enemigos/AI_Blueprints/NPC/NPC_BP/Animaciones/Combate/Montage/NPC_Reaction_hitFrom_Front_Montage.NPC_Reaction_hitFrom_Front_Montage" :`3` "/Game/Enemigos/AI_Blueprints/NPC/NPC_BP/Animaciones/Combate/Montage/NPC_Reaction_hitFrom_Right_Montage.NPC_Reaction_hitFrom_Right_Montage" :!type "AnimMontage Object Reference")))))

(event `MuerteNPC`
  ;[1 1 1] Muerte Porciacaso - No sirve
)

(event `Dano`
  ;[1 1 1] Dano Porciacaso (no sirve)
)

(fn `Ataque`
  (params (JoinInicio :type Name) (JoinFinal :type Name) (Radio :type "Float (double-precision)"))
  (bind _mesh (`self.Mesh`))
  (bind (_outhit _returnvalue) (`KismetSystemLibrary.SphereTraceSingle` :`Start` (`SceneComponent.GetSocketLocation` _mesh JoinInicio) :`End` (+ (`SceneComponent.GetSocketLocation` _mesh JoinFinal) (0.001 0.001 0.001)) :`Radius` Radio :`TraceChannel` "TraceTypeQuery2" :`DrawDebugType` "ForDuration"))
  (if _returnvalue
    (bind _asplayer_bp (cast `/Game/Jugador/PersonajePrincipal_Fausto/Blueprints/Character/Player_BP` (`.HitActor` (`GameplayStatics.BreakHitResult` _outhit))))
    (`GameplayStatics.ApplyDamage` _asplayer_bp 25.0 (`self.GetInstigatorController` (`Actor.Instigator` _asplayer_bp)) self "/Script/Engine.DamageType")))

(fn `UserConstructionScript`)