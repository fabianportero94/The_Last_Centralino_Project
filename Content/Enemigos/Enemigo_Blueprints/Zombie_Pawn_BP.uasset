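; Zombie enemy character that turns toward the player and deals melee damage.
; While FacePlayer is set, Tick interpolates its rotation toward the player's location.
; Atacar sphere-traces between right-hand mesh sockets on the Camera channel, with debug drawing, and damages any Player_BP hit.
; Helper functions set walk speed and expose its TargetPoints; some unconnected temporary attack and damage nodes remain.
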(event `InterpolarRotacion`
  (params (DeltaSeconds :type "Float (double-precision)"))
  ;[1 1 1] Interpola la velocidad con la que rota el enemigo hacia el jugador
  (set `self.Delta` DeltaSeconds)
  (if (`self.FacePlayer`)
    (`self.K2_SetActorRotation` self (`KismetMathLibrary.RInterpTo` (`self.K2_GetActorRotation` self) (`KismetMathLibrary.FindLookAtRotation` (`self.K2_GetActorLocation` self) (`self.K2_GetActorLocation` (`GameplayStatics.GetPlayerCharacter` 0))) (`self.Delta`) 50.0) false)))

(event `self.ReceiveTick`
  (params (DeltaSeconds :type "Float (single-precision)"))
  ;[1 1 1] Lanzar eventos Tick
  (`self.InterpolarRotacion` DeltaSeconds))

(event `Atacar`
  ;[1 1 1] Ataque al Jugador
  (bind (_outhit _returnvalue) (`KismetSystemLibrary.SphereTraceSingle` :`Start` (`SceneComponent.GetSocketLocation` (`self.Mesh`) "RightHand") :`End` (+ (`SceneComponent.GetSocketLocation` (`self.Mesh`) "RightHandMiddle4") (0.001 0.001 0.001)) :`Radius` 10.0 :`TraceChannel` "TraceTypeQuery2" :`DrawDebugType` "ForDuration"))
  (if _returnvalue
    (bind _asplayer_bp (cast `/Game/Jugador/PersonajePrincipal_Fausto/Blueprints/Character/Player_BP` (`.HitActor` (`GameplayStatics.BreakHitResult` _outhit))))
    (`GameplayStatics.ApplyDamage` _asplayer_bp 25.0 (`self.GetInstigatorController` (`Actor.Instigator` _asplayer_bp)) self "/Script/Engine.DamageType")))

(fn `Actualizar_Velocidad`
  (params (Nueva_Velocidad :type "Float (double-precision)"))
  (set `CharacterMovementComponent.MaxWalkSpeed` Nueva_Velocidad (`self.CharacterMovement`)))

(fn `ObtenerPuntos`
  (returns (TargetPoints :type "Array of TargetPoint Object Reference"))
  (return (`self.TargetPoints`)))

(fn `UserConstructionScript`)