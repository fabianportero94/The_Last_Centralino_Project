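; Mufi zombie enemy character that patrols around its spawn point and chases and attacks the player.
; Patrol walks to random line-traced points; PawnSensing starts a faster AIMoveTo chase with an attack montage, and a retriggerable delay resumes patrol.
; AtaqueMufi applies damage through a left-hand sphere trace.
; Dano updates the health-bar widget from SaludEnemigo, or ragdolls the body and hides the bar at zero health.
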(event `CambiarVelocidad`
  (params (Velocidad :type "Float (double-precision)"))
  (set `CharacterMovementComponent.MaxWalkSpeed` Velocidad (`self.CharacterMovement`)))

(event `self.ReceiveBeginPlay`
  (set `self.UbicacionInicial` (`self.K2_GetActorLocation`))
  (`self.Patrullaje`))

(event `self.ReceiveTick`
  (params (DeltaSeconds :type "Float (single-precision)"))
  (`KismetSystemLibrary.PrintString` (`KismetStringLibrary.Conv_DoubleToString` (`self.SaludEnemigo`)) true true (struct :`R` 1.0 :`B` 0.031609 :`A` 1.0) 0.0))

(event `Patrullaje`
  (bind (_ubicacioninicial_x _ubicacioninicial_y) (`KismetMathLibrary.BreakVector` (`self.UbicacionInicial`)))
  (bind _returnvalue (+ (`KismetMathLibrary.RandomFloatInRange` (* (`self.RadioMovimiento`) -1.0) (`self.RadioMovimiento`)) _ubicacioninicial_y))
  (bind _returnvalue_2 (+ (`KismetMathLibrary.RandomFloatInRange` (* (`self.RadioMovimiento`) -1.0) (`self.RadioMovimiento`)) _ubicacioninicial_x))
  ;[1 1 1] Patrullar
  (`self.CambiarVelocidad` 70.0)
  (bind _outhit (`KismetSystemLibrary.LineTraceSingle` :`Start` (`KismetMathLibrary.MakeVector` _returnvalue_2 _returnvalue 125.0) :`End` (`KismetMathLibrary.MakeVector` _returnvalue_2 _returnvalue) :`TraceChannel` "TraceTypeQuery1" :`DrawDebugType` "ForDuration" :`DrawTime` 20.0 :!label _label))
  (`|AIMoveTo` self (`.ImpactPoint` (`GameplayStatics.BreakHitResult` _outhit)) null
    (:`OnSuccess`
      (`KismetSystemLibrary.Delay` 2.0)
      (goto _label))))

(event `self.ReceiveAnyDamage`
  (params (Damage :type "Float (single-precision)") (DamageType :type "DamageType Object Reference") (InstigatedBy :type "Controller Object Reference") (DamageCauser :type "Actor Object Reference")))

(event `Dano`
  (bind _mesh (`self.Mesh`))
  (bind _capsulecomponent (`self.CapsuleComponent`))
  (if (> (`self.SaludEnemigo`) 0.0)
    (bind _asbarra_salud_enemigo (cast `/Game/Enemigos/Enemigo_Blueprints/BarraSaludEnemigo` (`WidgetComponent.GetUserWidgetObject` (`self.Widget`))))
    (`ProgressBar.SetPercent` (`/Game/Enemigos/Enemigo_Blueprints/BarraSaludEnemigo.ProgressBar_254` _asbarra_salud_enemigo) (/ (`self.SaludEnemigo`) 100.0))
    (else
      (`PrimitiveComponent.SetSimulatePhysics` _capsulecomponent true)
      (`PrimitiveComponent.SetCollisionResponseToChannel` _capsulecomponent "ECC_PhysicsBody" "ECR_Ignore")
      (`SkeletalMeshComponent.SetAllBodiesBelowSimulatePhysics` _mesh (`SkinnedMeshComponent.GetBoneName` _mesh 1) true true)
      (`SceneComponent.SetVisibility` (`self.Widget`) false false))))

(event `self.PawnSensing.OnSeePawn`
  (params (Pawn :type "Pawn Object Reference"))
  (bind _returnvalue (`AnimInstance.IsAnyMontagePlaying` (`SkeletalMeshComponent.GetAnimInstance` (`self.Mesh`))))
  ;[1 1 1] PawnSensing
  (bind _asplayer_bp (cast `/Game/Jugador/PersonajePrincipal_Fausto/Blueprints/Character/Player_BP` Pawn))
  (`self.CambiarVelocidad` 100.0)
  (if _returnvalue
    (`KismetSystemLibrary.RetriggerableDelay` 2.0 :!label _label_2)
    (`self.Patrullaje`)
    (else
      (`|AIMoveTo` self (0.0 0.0 0.0) _asplayer_bp 70.0
        (:`then`
          (goto _label_2))
        (:`OnSuccess`
          (if (not _returnvalue)
            (`|PlayMontage` (`self.Mesh`) "/Game/Enemigos/Mufi/Mixamo/MufiZombie_Attack_Montage.MufiZombie_Attack_Montage")))))))

(event `AtaqueMufi`
  (bind _returnvalue (`SceneComponent.GetSocketLocation` (`self.Mesh`) "LeftHandIndex2"))
  (bind (_outhit _returnvalue_2) (`KismetSystemLibrary.SphereTraceSingle` :`Start` _returnvalue :`End` (+ _returnvalue (0.1 0.1 0.1)) :`Radius` 25.0 :`TraceChannel` "TraceTypeQuery2" :`DrawDebugType` "ForDuration"))
  (if _returnvalue_2
    (`GameplayStatics.ApplyDamage` (`.HitActor` (`GameplayStatics.BreakHitResult` _outhit)) 10.0 (`self.GetInstigatorController` (`.HitActor` (`GameplayStatics.BreakHitResult` _outhit))) self)))

(fn `UserConstructionScript`)